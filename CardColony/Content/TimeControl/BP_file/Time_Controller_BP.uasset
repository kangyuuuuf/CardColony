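; Time controller that runs the game's day cycle, showing elapsed time and day count on a TimeBar widget.
; Tick advances the day and the timers in Timeset, removing finished ones, while Space toggles the clock.
; At day's end it shows a DayEndFade widget with the game paused, then starts the next day.
; It also calls RTS_Controller's RemoveRequiement, returning to Startmenu if that returns true.
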(event `self.ReceiveBeginPlay`
  ;[1 1 1] Preparation of the Day
  (bind _returnvalue (`|CreateWidget` "/Game/TimeControl/Widget_file/TimeBar.TimeBar_C"))
  (bind _output_get (set `self.TimeBar_Widget` _returnvalue))
  (`UserWidget.AddToViewport` _output_get 0)
  (`self.TimeCycle`))

(event `TimeCycle`
  ;[1 1 1] The cycle of the day
  (`self.DayStart`))

(event `DayStart`
  ;[1 1 1] Set the variable at the beginning of the day
  (bind _output_get (set `self.DayPassTime` 0.0))
  (set `/Game/TimeControl/Widget_file/TimeBar.TimePass` _output_get (`self.TimeBar_Widget`))
  (bind _output_get_2 (set `self.DayCount` (+ (`self.DayCount`) 1)))
  (set `/Game/TimeControl/Widget_file/TimeBar.DayNumber` _output_get_2 (`self.TimeBar_Widget`))
  (set `self.IsStop` false))

(event `self.ReceiveTick`
  (params (DeltaSeconds :type "Float (single-precision)"))
  ;[1 1 1] Time Track
  (if (not (`GameplayStatics.IsGamePaused`))
    (`self.pause`)
    (if (not (`self.IsStop`))
      (bind _output_get (set `self.DayPassTime` (+ DeltaSeconds (`self.DayPassTime`))))
      (bind _output_get_2 (set `/Game/TimeControl/Widget_file/TimeBar.TimePass` (/ _output_get (`self.DayLength`)) (`self.TimeBar_Widget`)))
      (`self.CheckTimeBar` DeltaSeconds)
      (if (>= _output_get_2 1.0)
        ;[1 1 1] The cycle of the day
        (`self.DayEnd`)))))

(event `DayEnd`
  ;[1 1 1] Set the variable at the end of day
  (set `self.IsStop` true)
  (`self.EndOfDay`)
  (`KismetSystemLibrary.Delay` 2.0)
  (`self.TimeCycle`)
  (bind _asrts_controller (cast `/Game/Traversal/ControlAndCamera/RTS_Controller` (`GameplayStatics.GetPlayerController` 0)))
  (bind _end (`/Game/Traversal/ControlAndCamera/RTS_Controller.RemoveRequiement` _asrts_controller))
  (if _end
    (`KismetSystemLibrary.Delay` 3.0)
    (`GameplayStatics.OpenLevel` "Startmenu")))

(event `pause`
  (if (`PlayerController.WasInputKeyJustPressed` (`GameplayStatics.GetPlayerController` 0) "SpaceBar")
    (set `self.IsStop` (not (`self.IsStop`)))))

(event `EndOfDay`
  (bind _returnvalue (`|CreateWidget` "/Game/TimeControl/Widget_file/DayEndFade.DayEndFade_C"))
  (set `/Game/TimeControl/Widget_file/DayEndFade.Day Value` (`self.DayCount`) _returnvalue)
  (`UserWidget.AddToViewport` _returnvalue 0)
  (`/Game/TimeControl/Widget_file/DayEndFade.StartFade` _returnvalue)
  (`GameplayStatics.SetGamePaused` true)
  (`KismetSystemLibrary.Delay` 2.0)
  (`GameplayStatics.SetGamePaused` false)
  (`Widget.RemoveFromParent` _returnvalue))

(fn `CheckTimeBar`
  (params (`delta sec` :type "Float (double-precision)"))
  (locals (timebar :type "/Game/CardBP/genericCard_BP Object Reference"))
  (bind _timeset (`self.Timeset`))
  (bind _result (`BlueprintSetLibrary.Set_ToArray` _timeset))
  (for _array_element _result
    (bind _output_get (set `/Game/TimeControl/Widget_file/Timeprogress.CurrentTime` (+ (`/Game/TimeControl/Widget_file/Timeprogress.CurrentTime` _array_element) `delta sec`) _array_element))
    (if (>= (/ _output_get (`/Game/TimeControl/Widget_file/Timeprogress.TimeLength` _array_element)) 1.0)
      (`BlueprintSetLibrary.Set_Remove` _timeset _array_element))))

(fn `UserConstructionScript`)