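; HooomanDelivery deck Blueprint that delivers a new astronaut whenever the deck produces.
; It overrides DeckProduction to call GenerateAstronaut before running the parent deck's production logic.
; GenerateAstronaut spawns an Astronaut_AstronautBP at a random X/Y offset within RandCardRange of the deck, keeping the deck's Z height.
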(fn `DeckProduction`
  (`self.GenerateAstronaut`)
  (`parent.DeckProduction`))

(fn `GenerateAstronaut`
  (bind (_returnvalue_x _returnvalue_y _returnvalue_z) (`KismetMathLibrary.BreakVector` (`self.K2_GetActorLocation`)))
  (bind _randcardrange (`self.randCardRange`))
  (`|SpawnActorFromClass` "/Game/CardBP/Astronauts/Astronaut_AstronautBP.Astronaut_AstronautBP_C" (`KismetMathLibrary.MakeTransform` (`KismetMathLibrary.MakeVector` (`KismetMathLibrary.RandomFloatInRange` (- _returnvalue_x _randcardrange) (+ _returnvalue_x _randcardrange)) (`KismetMathLibrary.RandomFloatInRange` (- _returnvalue_y _randcardrange) (+ _returnvalue_y _randcardrange)) _returnvalue_z)) "Undefined" "OverrideRootScale" null null))

(fn `UserConstructionScript`
  (`parent.UserConstructionScript`))