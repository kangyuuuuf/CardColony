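; Generic card deck actor that, when clicked, bursts into a random number of spawned cards and destroys itself.
; The click shakes the deck with delayed random XY offsets, then runs DeckProduction and plays a win sound.
; Each card's class comes from Production, picked by accumulating Probablity weights against a random threshold re-rolled at every step.
; Cards spawn at random XY positions within RandCardRange of the deck.
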(event `self.ReceiveTick`
  (params (DeltaSeconds :type "Float (single-precision)")))

(event `self.ReceiveBeginPlay`)

(event `self.Card.OnClicked`
  (params (TouchedComponent :type "PrimitiveComponent Object Reference") (ButtonPressed :type "Key Structure"))
  ;[1 1 1] Create Shaking Effect
  (`/Game/Traversal/ControlAndCamera/MyMacroLibrary.ForLoopWithDelay` 0 10 0.04
    (:`LoopBody`
      (`self.K2_AddActorLocalOffset` (`KismetMathLibrary.MakeVector` (`KismetMathLibrary.RandomFloatInRange` -50.0 50.0) (`KismetMathLibrary.RandomFloatInRange` -50.0 50.0))))
    (:`Completed`
      (`KismetSystemLibrary.Delay` 0.1)
      (`self.DeckProduction`)
      (`GameplayStatics.PlaySound2D` "/Game/Sounds/WAV/Win_V2.Win_V2" 1.0 1.0 0.0 null null))))

(event `self.Card.OnReleased`
  (params (TouchedComponent :type "PrimitiveComponent Object Reference") (ButtonReleased :type "Key Structure")))

(fn `DeckProduceOneCard`
  (bind (_returnvalue_x _returnvalue_y _returnvalue_z) (`KismetMathLibrary.BreakVector` (`self.K2_GetActorLocation`)))
  (bind _randcardrange (`self.randCardRange`))
  (bind _indexofcreation (`self.weightedProbabilityGeneration`))
  (`|SpawnActorFromClass` (`|GetArrayItem` (`self.Production`) _indexofcreation) (`KismetMathLibrary.MakeTransform` (`KismetMathLibrary.MakeVector` (`KismetMathLibrary.RandomFloatInRange` (- _returnvalue_x _randcardrange) (+ _returnvalue_x _randcardrange)) (`KismetMathLibrary.RandomFloatInRange` (- _returnvalue_y _randcardrange) (+ _returnvalue_y _randcardrange)) _returnvalue_z)) "Undefined" "OverrideRootScale" null null))

(fn `DeckProduction`
  (for _ (range 1 (+ (`KismetMathLibrary.RandomIntegerInRange` (`self.CardNumLowerBound`) (`self.CardNumUpperBound`)) 1))
    (`self.DeckProduceOneCard`))
  (`self.K2_DestroyActor`))

(fn `SumofArray`
  (returns (SumOfArray :type "Float (double-precision)"))
  (locals (tmep :type "Float (double-precision)"))
  (for _array_element (`self.Probablity`)
    (set `local.tmep` (+ _array_element (`local.tmep`))))
  (return (`local.tmep`)))

(fn `UserConstructionScript`)

(fn `weightedProbabilityGeneration`
  (returns (IndexOfCreation :type Integer))
  (locals (tempSum :type "Float (double-precision)" :default 0.0) (arrSum :type "Float (double-precision)"))
  (bind _sumofarray (`self.SumofArray`))
  (set `local.arrSum` _sumofarray)
  (set `local.tempSum` 0.0)
  (for (_array_element _array_index) (`self.Probablity`)
    (bind _output_get (set `local.tempSum` (+ _array_element (`local.tempSum`))))
    (if (>= _output_get (`KismetMathLibrary.RandomFloatInRange` 0.0 (`local.arrSum`)))
      (break)))
  (return _array_index))