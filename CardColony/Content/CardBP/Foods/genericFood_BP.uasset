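; Generic food card Blueprint that keeps the food count in the player's resource UI in step with its own lifetime.
; BeginPlay runs the parent logic, then casts player controller 0 to RTS_Controller and increments food on its ResourceWidget.
; EndPlay decrements food through the same widget, without calling the parent event.
; The count is updated directly on the widget, with no other logic in this Blueprint.
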(event `self.ReceiveBeginPlay`
  (`parent.ReceiveBeginPlay`)
  (bind _asrts_controller (cast `/Game/Traversal/ControlAndCamera/RTS_Controller` (`GameplayStatics.GetPlayerController` 0)))
  (`/Game/TimeControl/Widget_file/ResourceInfo.increamentfood` (`/Game/Traversal/ControlAndCamera/RTS_Controller.resourceWidget` _asrts_controller)))

(event `self.ReceiveEndPlay`
  (params (EndPlayReason :type "EEndPlayReason Enum" :default "Destroyed"))
  (bind _asrts_controller (cast `/Game/Traversal/ControlAndCamera/RTS_Controller` (`GameplayStatics.GetPlayerController` 0)))
  (`/Game/TimeControl/Widget_file/ResourceInfo.decreamentfood` (`/Game/Traversal/ControlAndCamera/RTS_Controller.resourceWidget` _asrts_controller)))

(fn `UserConstructionScript`
  (`parent.UserConstructionScript`))