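; Drinkable water Blueprint from the card food set that counts toward the player's water resource while it exists in the world.
; On BeginPlay it runs the parent logic, then casts player controller 0 to RTS_Controller and increments water on its ResourceWidget.
; On EndPlay it decrements the same counter through the controller, tying the tally directly to actor lifetime.
; Overlap and Tick only forward to the parent.
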(event `self.ReceiveBeginPlay`
  (`parent.ReceiveBeginPlay`)
  (bind _asrts_controller (cast `/Game/Traversal/ControlAndCamera/RTS_Controller` (`GameplayStatics.GetPlayerController` 0)))
  (`/Game/TimeControl/Widget_file/ResourceInfo.increamentwater` (`/Game/Traversal/ControlAndCamera/RTS_Controller.resourceWidget` _asrts_controller)))

(event `self.ReceiveActorBeginOverlap`
  (params (OtherActor :type "Actor Object Reference"))
  (`parent.ReceiveActorBeginOverlap` OtherActor))

(event `self.ReceiveTick`
  (params (DeltaSeconds :type "Float (single-precision)"))
  (`parent.ReceiveTick` DeltaSeconds))

(event `self.ReceiveEndPlay`
  (params (EndPlayReason :type "EEndPlayReason Enum" :default "Destroyed"))
  (bind _asrts_controller (cast `/Game/Traversal/ControlAndCamera/RTS_Controller` (`GameplayStatics.GetPlayerController` 0)))
  (`/Game/TimeControl/Widget_file/ResourceInfo.decreamentwater` (`/Game/Traversal/ControlAndCamera/RTS_Controller.resourceWidget` _asrts_controller)))

(fn `UserConstructionScript`)