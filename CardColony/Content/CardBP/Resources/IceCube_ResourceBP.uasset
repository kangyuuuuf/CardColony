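; IceCube_ResourceBP is an ice cube card resource that turns into a product card when IceProduction runs.
; IceProduction spawns a class from Production at a random XY offset within CardGenRange, removes itself from the 2D card array and destroys itself.
; The index comes from a weighted-probability loop over Probabilities, though its break test compares zero, not the running sum, to a random float.
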(fn `IceProduction`
  (locals (cardGenRange :type "Float (double-precision)" :default 400.0))
  (bind (_returnvalue_x _returnvalue_y _returnvalue_z) (`KismetMathLibrary.BreakVector` (`self.K2_GetActorLocation`)))
  (bind _cardgenrange (`local.cardGenRange`))
  (bind _indexofcreation (`self.Weighted Probability Generation`))
  (`|SpawnActorFromClass` (`|GetArrayItem` (`self.Production`) _indexofcreation) (`KismetMathLibrary.MakeTransform` (`KismetMathLibrary.MakeVector` (`KismetMathLibrary.RandomFloatInRange` (- _returnvalue_x _cardgenrange) (+ _returnvalue_x _cardgenrange)) (`KismetMathLibrary.RandomFloatInRange` (- _returnvalue_y _cardgenrange) (+ _returnvalue_y _cardgenrange)) _returnvalue_z)) "Undefined" "OverrideRootScale" null null)
  (`self.RemoveTargetCardFrom2DArray` self self)
  (`self.K2_DestroyActor`))

(fn `UserConstructionScript`
  (`parent.UserConstructionScript`))

(fn `Weighted Probability Generation`
  (returns (IndexOfCreation :type Integer))
  (locals (tempSum :type "Float (double-precision)" :default 0.0))
  (set `local.tempSum` 0.0)
  (for (_array_element _array_index) (`self.Probabilities`)
    (set `local.tempSum` (+ _array_element (`local.tempSum`)))
    (if (>= 0.0 (`KismetMathLibrary.RandomFloat`))
      (break)))
  (return _array_index))