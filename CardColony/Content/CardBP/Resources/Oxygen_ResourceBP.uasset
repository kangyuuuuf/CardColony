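; Oxygen resource actor Blueprint that adjusts the player's oxygen readout for as long as it exists in the world.
; On BeginPlay it gets player 0's RTS_Controller and increments oxygen on its ResourceWidget.
; On EndPlay it calls the matching decrement, so the change is tied directly to the actor's lifetime and made through the UI widget.
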(event `self.ReceiveBeginPlay`
  (`parent.ReceiveBeginPlay`)
  (bind _asrts_controller (cast `/Game/Traversal/ControlAndCamera/RTS_Controller` (`GameplayStatics.GetPlayerController` 0)))
  (`/Game/TimeControl/Widget_file/ResourceInfo.increamentoxygen` (`/Game/Traversal/ControlAndCamera/RTS_Controller.resourceWidget` _asrts_controller)))

(event `self.ReceiveEndPlay`
  (params (EndPlayReason :type "EEndPlayReason Enum" :default "Destroyed"))
  (`parent.ReceiveEndPlay` EndPlayReason)
  (bind _asrts_controller (cast `/Game/Traversal/ControlAndCamera/RTS_Controller` (`GameplayStatics.GetPlayerController` 0)))
  (`/Game/TimeControl/Widget_file/ResourceInfo.decreamentoxygen` (`/Game/Traversal/ControlAndCamera/RTS_Controller.resourceWidget` _asrts_controller)))

(fn `UserConstructionScript`
  (`parent.UserConstructionScript`))