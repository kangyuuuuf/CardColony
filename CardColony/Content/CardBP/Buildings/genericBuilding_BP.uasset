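; Generic building Blueprint for a card-based game that produces cards by spawning them as actors around itself.
; BuildingProduction loops over the Production list and passes each entry to BuildingProduceSingleCard.
; Each card spawns at a random X/Y within CardProductionRange of the building, in a square area at the building's height.
; The event graph holds only disabled default events, so nothing in this Blueprint triggers production itself.
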(fn `BuildingProduceSingleCard`
  (params (CardRef :type "/Game/CardBP/genericCard_BP Class Reference"))
  (bind (_returnvalue_x _returnvalue_y _returnvalue_z) (`KismetMathLibrary.BreakVector` (`self.K2_GetActorLocation`)))
  (bind _cardproductionrange (`self.cardProductionRange`))
  (`|SpawnActorFromClass` CardRef (`KismetMathLibrary.MakeTransform` (`KismetMathLibrary.MakeVector` (`KismetMathLibrary.RandomFloatInRange` (- _returnvalue_x _cardproductionrange) (+ _returnvalue_x _cardproductionrange)) (`KismetMathLibrary.RandomFloatInRange` (- _returnvalue_y _cardproductionrange) (+ _returnvalue_y _cardproductionrange)) _returnvalue_z)) "Undefined" "OverrideRootScale" null null))

(fn `BuildingProduction`
  (for _array_element (`self.Production`)
    (`self.BuildingProduceSingleCard` _array_element)))

(fn `UserConstructionScript`
  (`parent.UserConstructionScript`))