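; Generic card container actor that holds a one-dimensional array of cards.
; Functions add or remove a given card, and a print function joins the names of valid cards into a comma-delimited debug string.
; Its event graph and construction script are empty, so the array changes only when these functions or other code act on it.
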(fn `1DArrayAdd`
  (params (CardToAdd :type "/Game/CardBP/genericCard_BP Object Reference"))
  (`KismetArrayLibrary.Array_Add` (`self.Card1DArray`) CardToAdd))

(fn `1DArrayPrint`
  (set `self.cardString` "")
  (for _array_element (`self.Card1DArray`)
    (`/Engine/EditorBlueprintResources/StandardMacros.IsValid` _array_element
      (:`Is Valid`
        (set `self.cardString` (`KismetStringLibrary.Concat_StrStr` (`self.cardString`) (`KismetStringLibrary.Conv_NameToString` (`/Game/CardBP/genericCard_BP.CardName` _array_element)) ", ")))))
  (`KismetSystemLibrary.PrintString` (`self.cardString`)))

(fn `1DArrayRemove`
  (params (CardToRemove :type "/Game/CardBP/genericCard_BP Object Reference"))
  (`KismetArrayLibrary.Array_RemoveItem` (`self.Card1DArray`) CardToRemove))

(fn `UserConstructionScript`)