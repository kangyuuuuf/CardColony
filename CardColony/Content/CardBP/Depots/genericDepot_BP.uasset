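; Generic depot card that produces other cards nearby and has a limited number of uses.
; DepotProduction picks a class from Production by cumulative Probability weights, re-rolling the random value at each step, and spawns it at a random X/Y offset within CardProductionRange.
; Each production spends a use; at zero, the depot removes itself from the card 2D array and is destroyed.
; The event graph's mouse-gated DepotProduction call is disconnected.
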(event `self.ReceiveBeginPlay`
  (`parent.ReceiveBeginPlay`))

(event `self.ReceiveTick`
  (params (DeltaSeconds :type "Float (single-precision)"))
  (`parent.ReceiveTick` DeltaSeconds))

(fn `CheckUses`
  (if (<= (`self.Uses`) 0)
    (`self.RemoveTargetCardFrom2DArray` self)
    (`self.K2_DestroyActor`)))

(fn `DepotProduction`
  (bind (_returnvalue_x _returnvalue_y _returnvalue_z) (`KismetMathLibrary.BreakVector` (`self.K2_GetActorLocation`)))
  (bind _cardproductionrange (`self.cardProductionRange`))
  (bind _indexofcreation (`self.weightedProbabilityGeneration`))
  (`|SpawnActorFromClass` (`|GetArrayItem` (`self.Production`) _indexofcreation) (`KismetMathLibrary.MakeTransform` (`KismetMathLibrary.MakeVector` (`KismetMathLibrary.RandomFloatInRange` (- _returnvalue_x _cardproductionrange) (+ _returnvalue_x _cardproductionrange)) (`KismetMathLibrary.RandomFloatInRange` (- _returnvalue_y _cardproductionrange) (+ _returnvalue_y _cardproductionrange)) _returnvalue_z)) "Undefined" "OverrideRootScale" null null)
  (`/Engine/EditorBlueprintResources/StandardMacros.DecrementInt` (`self.Uses`)
    (:`  `
      (`self.CheckUses`))))

(fn `UserConstructionScript`
  (`parent.UserConstructionScript`))

(fn `weightedProbabilityGeneration`
  (returns (IndexOfCreation :type Integer))
  (locals (tempSum :type "Float (double-precision)"))
  (set `local.tempSum` 0.0)
  (for (_array_element _array_index) (`self.Probability`)
    (bind _output_get (set `local.tempSum` (+ _array_element (`local.tempSum`))))
    (if (>= _output_get (`KismetMathLibrary.RandomFloat`))
      (break)))
  (return _array_index))