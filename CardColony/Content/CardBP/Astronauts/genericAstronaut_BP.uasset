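; Generic astronaut actor for an RTS-style card game, with hit points shown on a text display.
; BeginPlay fills HP to max and raises the Population count on the RTS controller's resource widget; EndPlay lowers and prints it.
; Tick refreshes the HP text and destroys the actor when HP runs out or it is no longer alive.
; An unconnected branch that drains HP while the left mouse is held never runs.
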(event `self.ReceiveBeginPlay`
  (`parent.ReceiveBeginPlay`)
  (set `self.currentHP` (`self.maxHP`))
  (`self.UpdateHPRender`)
  (bind _asrts_controller (cast `/Game/Traversal/ControlAndCamera/RTS_Controller` (`GameplayStatics.GetPlayerController` 0)))
  (`/Engine/EditorBlueprintResources/StandardMacros.IncrementInt` (`/Game/TimeControl/Widget_file/ResourceInfo.population` (`/Game/Traversal/ControlAndCamera/RTS_Controller.resourceWidget` _asrts_controller))))

(event `self.ReceiveTick`
  (params (DeltaSeconds :type "Float (single-precision)"))
  (`parent.ReceiveTick` DeltaSeconds)
  (if (or (<= (`self.currentHP`) 0) (not (`self.isAlive`)))
    (`self.K2_DestroyActor`)
    (else
      (`self.UpdateHPRender`))))

(event `self.ReceiveEndPlay`
  (params (EndPlayReason :type "EEndPlayReason Enum" :default "Destroyed"))
  (`parent.ReceiveEndPlay` EndPlayReason)
  (bind _asrts_controller (cast `/Game/Traversal/ControlAndCamera/RTS_Controller` (`GameplayStatics.GetPlayerController` 0)))
  (bind _result (`/Engine/EditorBlueprintResources/StandardMacros.DecrementInt` (`/Game/TimeControl/Widget_file/ResourceInfo.population` (`/Game/Traversal/ControlAndCamera/RTS_Controller.resourceWidget` _asrts_controller)))
    (:`  `
      (`KismetSystemLibrary.PrintString` (`KismetStringLibrary.Conv_IntToString` _result)))))

(fn `UpdateHPRender`
  (`TextRenderComponent.K2_SetText` (`self.HPRender`) (`KismetTextLibrary.Conv_IntToText` (`self.currentHP`))))

(fn `UserConstructionScript`
  (`parent.UserConstructionScript`)
  (`self.UpdateHPRender`))